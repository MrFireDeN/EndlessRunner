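; BP_MainGI is a game instance that keeps the player's selected character and score record across sessions.
; On Init it loads the "save" slot into a BP_SaveGame and restores both values, or creates and saves a new one from its current values.
; SaveRecord writes a score only when it beats the stored record.
; SaveSelectedCharacter writes the character choice to the slot immediately.
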(event Custom|SaveRecord
  (params (Record :type Float%20%28double-precision%29))
  (bind _savegame (Variables|Default|GetSaveGame))
  (if (> Record (Variables|Default|GetScoreRecord))
    (bind _output_get (Variables|Default|SetScoreRecord Record))
    (Variables|/Game/Project/Blueprints/BP_SaveGame.BP_SaveGame_C|SetScoreRecord _savegame _output_get)
    (SaveGame|SaveGametoSlot _savegame "save")))

(event Custom|SaveSelectedCharacter
  (params (SelectedCharacter :type BP%20Character%20Class%20Reference))
  (bind _savegame (Variables|Default|GetSaveGame))
  (bind _output_get (Variables|Default|SetSelectedCharacter SelectedCharacter))
  (Variables|/Game/Project/Blueprints/BP_SaveGame.BP_SaveGame_C|SetLastCharater _savegame _output_get)
  (SaveGame|SaveGametoSlot _savegame "save"))

(event EventInit
  (bind _returnvalue (SaveGame|DoesSaveGameExist "save"))
  (if _returnvalue
    (bind _returnvalue_2 (SaveGame|LoadGamefromSlot "save"))
    (bind _asbp_save_game (Utilities|Casting|CastToBP_SaveGame _returnvalue_2))
    (bind _output_get (Variables|Default|SetSaveGame _asbp_save_game))
    (Variables|Default|SetSelectedCharacter (Variables|/Game/Project/Blueprints/BP_SaveGame.BP_SaveGame_C|GetLastCharater _output_get))
    (Variables|Default|SetScoreRecord (Variables|/Game/Project/Blueprints/BP_SaveGame.BP_SaveGame_C|GetScoreRecord _output_get))
    (else
      (bind _returnvalue_3 (SaveGame|CreateSaveGameObject "/Game/Project/Blueprints/BP_SaveGame.BP_SaveGame_C"))
      (bind _output_get_2 (Variables|Default|SetSaveGame _returnvalue_3))
      (Variables|/Game/Project/Blueprints/BP_SaveGame.BP_SaveGame_C|SetLastCharater _output_get_2 (Variables|Default|GetSelectedCharacter))
      (Variables|/Game/Project/Blueprints/BP_SaveGame.BP_SaveGame_C|SetScoreRecord _output_get_2 (Variables|Default|GetScoreRecord))
      (SaveGame|SaveGametoSlot (Variables|Default|GetSaveGame) "save"))))