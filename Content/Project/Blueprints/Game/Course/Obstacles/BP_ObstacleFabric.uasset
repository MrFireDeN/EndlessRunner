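; BP_ObstacleFabric is an obstacle factory that randomly populates road pieces in the course.
; Its GenerateObstacles event walks the given road's obstacle points, giving each a weighted chance to receive an obstacle.
; A coin flip picks the dodgeable or non-dodgeable class pool, and a random class from it is spawned at the point.
; Each spawned obstacle attaches to its point component, snapping to its location.
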(event Custom|GenerateObstacles
  (params (Road :type BP%20Road%20BASE%20Object%20Reference))
  (for _array_element (Variables|/Game/Project/Blueprints/Game/Course/BP_Road_BASE.BP_Road_BASE_C|GetObstaclePoints Road)
    (if (Math|Random|RandomBoolwithWeight 0.3)
      (bind _returnvalue (Game|SpawnActorfromClass (.OutItem (Utilities|Array|Random (select (Math|Random|RandomBool) (Variables|Default|GetNonDodgeableObstacles) (Variables|Default|GetDodgeableObstacles)))) (Transformation|GetWorldTransform _array_element) "Undefined" "MultiplyWithRoot" 0 0))
      (Transformation|AttachComponentToComponent _returnvalue _array_element "None" "SnapToTarget" "KeepRelative" "KeepRelative" true))))

(fn ConstructionScript)