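; BP_RoadFabric is a road spawner that keeps an endless track of BP_Road_BASE segments running along the X axis.
; On BeginPlay it spawns ten evenly spaced segments.
; When a road segment stops overlapping it, it spawns a replacement one full track length ahead of that segment's current X position.
; It destroys every actor that ends overlap, road or not, recycling by spawn and destroy rather than pooling.
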(event Custom|SpawnRoad
  ;[1 1 1] Spawn Road
  (for _index (range 0 9)
    (Game|SpawnActorfromClass "/Game/Project/Blueprints/Game/Course/BP_Road_BASE.BP_Road_BASE_C" (Math|Transform|MakeTransform (Math|Vector|MakeVector (Math|Conversions|ToFloat(Integer) (* _index 1500)) 0.0 0.0) "0, 0, 0" "1.000000,1.000000,1.000000") "Undefined" "MultiplyWithRoot" 0 0)))

(event Custom|UpdateRoad
  (params (Road :type Actor%20Object%20Reference))
  ;[1 1 1] UpdateRoad
  (bind _asbp_road_base (Utilities|Casting|CastToBP_Road_BASE Road))
  (Game|SpawnActorfromClass "/Game/Project/Blueprints/Game/Course/BP_Road_BASE.BP_Road_BASE_C" (Math|Transform|MakeTransform (Math|Vector|MakeVector (+ (.x (Transformation|GetActorLocation _asbp_road_base)) (* 1.5e+03 1e+01)) 0.0 0.0) "0, 0, 0" "1.000000,1.000000,1.000000") "Undefined" "MultiplyWithRoot" 0 0))

(event EventBeginPlay
  (CallFunction|SpawnRoad))

(event Collision|EventActorBeginOverlap
  (params (OtherActor :type Actor%20Object%20Reference)))

(event EventTick
  (params (DeltaSeconds :type Float%20%28single-precision%29)))

(event Collision|EventActorEndOverlap
  (params (OtherActor :type Actor%20Object%20Reference))
  (CallFunction|UpdateRoad OtherActor)
  (Actor|DestroyActor OtherActor))

(fn ConstructionScript)