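; BP_ObstacleFabric is a spawner that lays out a recycling row of course obstacles along the X axis.
; On BeginPlay it spawns ten BP_Obstacle_BASE actors at even X spacing.
; When an obstacle stops overlapping this actor, it is moved forward by the full row length, so the same pool repeats endlessly instead of spawning new ones.
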(event Custom|SpawnObstacle
  ;[1 1 1] Spawn Road
  (for _index (range 0 9)
    (Game|SpawnActorfromClass "/Game/Project/Blueprints/Game/Course/BP_Obstacle_BASE.BP_Obstacle_BASE_C" (Math|Transform|MakeTransform (Math|Vector|MakeVector (Math|Conversions|ToFloat(Integer) (* _index 1500)) 0.0 0.0) "0, 0, 0" "1.000000,1.000000,1.000000") "Undefined" "MultiplyWithRoot" 0 0)))

(event Custom|UpdateObstacle
  (params (Obstacle :type Actor%20Object%20Reference))
  (bind _asbp_obstacle_base (Utilities|Casting|CastToBP_Obstacle_BASE Obstacle))
  (Transformation|SetActorLocation _asbp_obstacle_base (Math|Vector|MakeVector (+ (.x (Transformation|GetActorLocation _asbp_obstacle_base)) (* 1.5e+03 1e+01)) 0.0 0.0) false false))

(event EventBeginPlay
  (CallFunction|SpawnObstacle))

(event Collision|EventActorBeginOverlap
  (params (OtherActor :type Actor%20Object%20Reference)))

(event EventTick
  (params (DeltaSeconds :type Float%20%28single-precision%29)))

(event Collision|EventActorEndOverlap
  (params (OtherActor :type Actor%20Object%20Reference))
  (CallFunction|UpdateObstacle OtherActor))

(fn ConstructionScript)