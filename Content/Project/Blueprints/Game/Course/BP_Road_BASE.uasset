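; BP_Road_BASE is a base road segment for a runner course that scrolls along negative X.
; On BeginPlay it caches the game state, gathers six center, left and right obstacle points, and spawns a BP_ObstacleFabric to generate obstacles on itself.
; Each Tick it shifts its location by the game state's RunnerSpeed scaled by delta time, so the road itself moves to create the running motion.
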(event EventBeginPlay
  (Variables|Default|SetAs%20BP%20Game%20State (.AsBP%20Game%20State (Utilities|Casting|CastToBP_GameState (Game|GetGameState))))
  (Variables|Default|SetObstaclePoints (Utilities|Array|MakeArray (Variables|Default|GetCenterObstacleBack) (Variables|Default|GetCenterObstacleForward) (Variables|Default|GetLeftObstacleBack) (Variables|Default|GetRightObstacleForward) (Variables|Default|GetLeftObstacleForward) (Variables|Default|GetRightObstacleBack)))
  (bind _returnvalue (Game|SpawnActorfromClass "/Game/Project/Blueprints/Game/Course/Obstacles/BP_ObstacleFabric.BP_ObstacleFabric_C" (Math|Transform|MakeTransform "0, 0, 0" "0, 0, 0" "1.000000,1.000000,1.000000") "Undefined" "MultiplyWithRoot" 0 0))
  (Default|GenerateObstacles _returnvalue self))

(event Collision|EventActorBeginOverlap
  (params (OtherActor :type Actor%20Object%20Reference)))

(event EventTick
  (params (DeltaSeconds :type Float%20%28single-precision%29))
  (bind _returnvalue (Transformation|GetActorLocation))
  (Transformation|SetActorLocation (Math|Vector|MakeVector (- (.x _returnvalue) (* DeltaSeconds (Variables|/Game/Project/Blueprints/Game/BP_GameState.BP_GameState_C|GetRunnerSpeed (Variables|Default|GetAs%20BP%20Game%20State)))) (.y _returnvalue) (.z _returnvalue)) false false))

(fn ConstructionScript)