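; BP_PlayerController is a player controller that manages the in-game HUD and the end-of-game screen.
; On BeginPlay it creates both widgets, adds only the HUD to the viewport and hides the mouse cursor.
; Its EndGame event pauses through the "pause" console command, adds the pre-created end screen to the viewport and shows the cursor.
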(event Custom|EndGame
  (Development|ExecuteConsoleCommand "pause" 0)
  (UserInterface|Viewport|AddtoViewport (Variables|Default|GetEnd%20Screen%20Widget) 0)
  (Variables|Default|SetbShowMouseCursor true))

(event EventBeginPlay
  (bind _returnvalue (UserInterface|CreateWidget "/Game/Project/UI/Game/WBP_HUD.WBP_HUD_C"))
  (bind _output_get (Variables|Default|SetHUD _returnvalue))
  (UserInterface|Viewport|AddtoViewport _output_get 0)
  (bind _returnvalue_2 (UserInterface|CreateWidget "/Game/Project/UI/Game/WBP_EndScreen.WBP_EndScreen_C"))
  (Variables|Default|SetEnd%20Screen%20Widget _returnvalue_2)
  (Variables|Default|SetbShowMouseCursor false))

(event EventTick
  (params (DeltaSeconds :type Float%20%28single-precision%29)))

(fn ConstructionScript)